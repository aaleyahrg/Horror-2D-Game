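; BP-Player is a player Blueprint that fires a short sphere trace forward from its camera on left mouse click, with debug drawing.
; The trace result currently drives nothing, as the branch after it is empty.
; Disconnected nodes would cast the hit actor to Cube_Blueprint and push its mesh along the camera's forward vector with AddForce, but they never run.
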(event `Key|LeftMouseButton`
  (params (Key :type "Key Structure"))
  (bind _camera (`self.Camera`))
  (bind _returnvalue (`SceneComponent.K2_GetComponentLocation` _camera))
  (:`Pressed`
    (bind _outhit (`KismetSystemLibrary.SphereTraceSingle` :`Start` _returnvalue :`End` (+ _returnvalue (* (`KismetMathLibrary.GetForwardVector` (`SceneComponent.K2_GetComponentRotation` _camera)) 200.0)) :`Radius` 15.0 :`TraceChannel` "TraceTypeQuery1" :`DrawDebugType` "ForDuration"))
    (if true
      _)))

(fn `UserConstructionScript`)